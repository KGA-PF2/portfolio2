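; BP_CharacterBase is a character base Blueprint whose live graphs are currently empty.
; BeginPlay, OnHPUpdated and the construction script do nothing.
; Disconnected nodes hold health bar logic that would initialize a WBP_HealthBar widget from Attributes, bind to health changes and hide a component at zero health, but none of it runs.
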(event `self.ReceiveBeginPlay`)

(event `OnHPUpdated` :!signature `self.OnHealthChanged`
  (params (NewHealth :type Integer) (NewMaxHealth :type Integer)))

(fn `UserConstructionScript`)