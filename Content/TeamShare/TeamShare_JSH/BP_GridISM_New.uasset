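; Grid actor that builds a flat tile grid from one instanced static mesh component at BeginPlay.
; It stores its root world location as an offset, then adds Plane instances in local space, scaled to cell size minus a gap.
; Helper functions expose grid dimensions and cell size, and convert between instance index and X/Y coordinate using X-major order (index = X * height + Y).
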(event `self.ReceiveBeginPlay`
  (bind _gridinstance (`self.GridInstance`))
  (bind _gridinterval (`self.GridInterval`))
  (set `self.GridLocationOffset` (`SceneComponent.K2_GetComponentLocation` (`self.DefaultSceneRoot`)))
  (`InstancedStaticMeshComponent.ClearInstances` _gridinstance)
  (`StaticMeshComponent.SetStaticMesh` _gridinstance "/Engine/BasicShapes/Plane.Plane")
  (for _index (range (`self.GridWidth`))
    (for _index_2 (range (`self.GridHeight`))
      (`InstancedStaticMeshComponent.AddInstance` _gridinstance (`KismetMathLibrary.MakeTransform` (`KismetMathLibrary.MakeVector` (* _index (`self.GridSizeX`)) (* _index_2 (`self.GridSizeY`)) 0.3) (struct) (`KismetMathLibrary.MakeVector` (/ (- (`self.GridSizeX`) _gridinterval) 100.0) (/ (- (`self.GridSizeY`) _gridinterval) 100.0) 0.1)) false))))

(fn `GetGridCoordFromIndex`
  (params (Index :type Integer))
  (returns (ReturnValue :type "IntPoint Structure"))
  (return (make `IntPoint` (/ Index (`self.GridHeight`)) (mod Index (`self.GridHeight`)))))

(fn `GetGridHeight`
  (returns (ReturnValue :type Integer))
  (return (`self.GridHeight`)))

(fn `GetGridIndexFromCoord`
  (params (Coord :type "IntPoint Structure (by ref)"))
  (returns (ReturnValue :type Integer))
  (return (+ (* Coord_X (`self.GridHeight`)) Coord_Y)))

(fn `GetGridSizeX`
  (returns (ReturnValue :type "Float (double-precision)"))
  (return (`self.GridSizeX`)))

(fn `GetGridSizeY`
  (returns (ReturnValue :type "Float (double-precision)"))
  (return (`self.GridSizeY`)))

(fn `GetGridWidth`
  (returns (ReturnValue :type Integer))
  (return (`self.GridWidth`)))

(fn `UserConstructionScript`)