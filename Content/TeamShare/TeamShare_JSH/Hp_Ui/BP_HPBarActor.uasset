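; BP_HPBarActor is an actor that displays health through a WBP_HealthBar widget held in its HPBarWidget component.
; Initialize and HandleHealthChanged each cast that widget and pass current and maximum HP to UpdateHealth.
; Every tick it interpolates its location toward TargetWorldLocation, which is not set within these graphs, so the bar glides to its target.
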(event `self.ReceiveTick`
  (params (DeltaSeconds :type "Float (single-precision)"))
  (`self.K2_SetActorLocation` (`KismetMathLibrary.VInterpTo` (`self.K2_GetActorLocation`) (`self.TargetWorldLocation`) DeltaSeconds)))

(event `HandleHealthChanged`
  (params (NewHealth :type Integer) (NewMaxHealth :type Integer))
  (bind _aswbp_health_bar (cast `/Game/TeamShare/TeamShare_JSH/Hp_Ui/WBP_HealthBar` (`WidgetComponent.GetUserWidgetObject` (`self.HPBarWidget`))))
  (`/Game/TeamShare/TeamShare_JSH/Hp_Ui/WBP_HealthBar.UpdateHealth` _aswbp_health_bar NewHealth NewMaxHealth))

(event `Initialize`
  (params (CurrentHP :type Integer) (MaxHP :type Integer))
  (bind _aswbp_health_bar (cast `/Game/TeamShare/TeamShare_JSH/Hp_Ui/WBP_HealthBar` (`WidgetComponent.GetUserWidgetObject` (`self.HPBarWidget`))))
  (`/Game/TeamShare/TeamShare_JSH/Hp_Ui/WBP_HealthBar.UpdateHealth` _aswbp_health_bar CurrentHP MaxHP))

(fn `UserConstructionScript`)