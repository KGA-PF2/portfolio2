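; BP_GroundGrid_New is a ground grid Blueprint that exposes grid dimensions and converts between linear cell indices and 2D coordinates.
; Index conversion is column-major: X is the index divided by GridHeight, Y is the remainder, and the inverse is X * GridHeight + Y.
; Getters return grid width, height and X/Y sizes.
; The event graph holds only disabled default events, and the construction script just calls its parent.
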(fn `GetGridCoordFromIndex`
  (params (Index :type Integer))
  (returns (ReturnValue :type "IntPoint Structure"))
  (return (make `IntPoint` (/ Index (`self.GridHeight`)) (mod Index (`self.GridHeight`)))))

(fn `GetGridHeight`
  (returns (ReturnValue :type Integer))
  (return (`self.GridHeight`)))

(fn `GetGridIndexFromCoord`
  (params (Coord :type "IntPoint Structure (by ref)"))
  (returns (ReturnValue :type Integer))
  (return (+ (* Coord_X (`self.GridHeight`)) Coord_Y)))

(fn `GetGridSizeX`
  (returns (ReturnValue :type "Float (double-precision)"))
  (return (`self.GridSizeX`)))

(fn `GetGridSizeY`
  (returns (ReturnValue :type "Float (double-precision)"))
  (return (`self.GridSizeY`)))

(fn `GetGridWidth`
  (returns (ReturnValue :type Integer))
  (return (`self.GridWidth`)))

(fn `UserConstructionScript`
  (`parent.UserConstructionScript`))