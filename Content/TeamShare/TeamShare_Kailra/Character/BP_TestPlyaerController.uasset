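; Test player controller that drives a BP_TestAIC actor around a BP_GridISM instanced-mesh grid and switches between level cameras.
; Arrow keys compute a target cell index through calcTargetGridNum, while Z, C and X step a separate index back, forward or randomly, feeding instance locations to MovingOn.
; A looping timer, rather than Tick, traces under the cursor to update grid hover.
; PageUp and PageDown blend between placed CameraActors.
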(event `Key|Up`
  (params (Key :type "Key Structure"))
  (bind _as_bp_gridism (`self.As BP GridISM`))
  ;[1 1 1] 위, 아래, 좌, 우 키 입력 기반으로 인스턴스 그리드 인덱스를 계산 플레이어 캐릭터 이동
  (:`Pressed`
    (bind (_calcgridnum _bsuccessout) (`NewFunctionLibrary.CalcTargetGridNum` (`self.Current Grid Num`) (`GridISM.GridWidth` _as_bp_gridism) (`GridISM.GridHeight` _as_bp_gridism) :!label _label))
    (if _bsuccessout
      (set `self.Current Grid Num` _calcgridnum)
      (`/Game/TeamShare/TeamShare_Kailra/Character/BP_TestAIC.MovingOn` (`self.TestAIC`) (`KismetMathLibrary.Conv_Vector2DToVector` (`KismetMathLibrary.Conv_VectorToVector2D` (+ (.location (`InstancedStaticMeshComponent.GetInstanceTransform` (`/Game/TeamShare/TeamShare_Kailra/Stage/StageBase/BP_GridISM.GridInstance` (`self.As BP GridISM`)) (`self.Current Grid Num`) false)) (`GridISM.GridLocationOffset` (`self.As BP GridISM`)))))))))

(event `Key|Down`
  (params (Key :type "Key Structure"))
  ;[1 1 1] 위, 아래, 좌, 우 키 입력 기반으로 인스턴스 그리드 인덱스를 계산 플레이어 캐릭터 이동
  (:`Pressed`
    (goto _label :!via `Down`)))

(event `Key|Left`
  (params (Key :type "Key Structure"))
  ;[1 1 1] 위, 아래, 좌, 우 키 입력 기반으로 인스턴스 그리드 인덱스를 계산 플레이어 캐릭터 이동
  (:`Pressed`
    (goto _label :!via `Left`)))

(event `Key|Right`
  (params (Key :type "Key Structure"))
  ;[1 1 1] 위, 아래, 좌, 우 키 입력 기반으로 인스턴스 그리드 인덱스를 계산 플레이어 캐릭터 이동
  (:`Pressed`
    (goto _label :!via `Right`)))

(event `Key|Z`
  (params (Key :type "Key Structure"))
  ;[1 1 1] Grid 순회 Z = -1, C = +1, X = Random
  (:`Pressed`
    (`/Engine/EditorBlueprintResources/StandardMacros.DecrementInt` (`self.InstanceIndexNum`)
      (:`  `
        (if (>= (`self.InstanceIndexNum`) 0.0)
          (`/Game/TeamShare/TeamShare_Kailra/Character/BP_TestAIC.MovingOn` (`self.TestAIC`) (+ (.location (`InstancedStaticMeshComponent.GetInstanceTransform` (`/Game/TeamShare/TeamShare_Kailra/Stage/StageBase/BP_GridISM.GridInstance` (`self.As BP GridISM`)) (`self.InstanceIndexNum`) false)) (`GridISM.GridLocationOffset` (`self.As BP GridISM`))) :!label _label_2)
          (else
            (set `self.InstanceIndexNum` 0)))))))

(event `Key|X`
  (params (Key :type "Key Structure"))
  (bind _as_bp_gridism (`self.As BP GridISM`))
  ;[1 1 1] Grid 순회 Z = -1, C = +1, X = Random
  (:`Pressed`
    (set `self.InstanceIndexNum` (`KismetMathLibrary.RandomIntegerInRange` 1 (- (* (`GridISM.GridWidth` _as_bp_gridism) (`GridISM.GridHeight` _as_bp_gridism)) 2)))
    (goto _label_2)))

(event `Key|C`
  (params (Key :type "Key Structure"))
  (bind _as_bp_gridism (`self.As BP GridISM`))
  (bind _returnvalue (- (* (`GridISM.GridWidth` _as_bp_gridism) (`GridISM.GridHeight` _as_bp_gridism)) 1))
  ;[1 1 1] Grid 순회 Z = -1, C = +1, X = Random
  (:`Pressed`
    (`/Engine/EditorBlueprintResources/StandardMacros.IncrementInt` (`self.InstanceIndexNum`)
      (:`  `
        (if (<= (`self.InstanceIndexNum`) _returnvalue)
          (goto _label_2)
          (else
            (set `self.InstanceIndexNum` _returnvalue)))))))

(event `Possess Event`
  (params (InPawn :type "Pawn Object Reference"))
  (`self.Possess` InPawn))

(event `Key|PageDown`
  (params (Key :type "Key Structure"))
  (:`Pressed`
    (if (!= (+ (`KismetArrayLibrary.Array_Find` (`self.CameraActors`)) 1) (`self.CameraNum`))
      (set `self.CameraNum` (- (`self.CameraNum`) 1))
      (`self.SetViewTargetWithBlend` (`|GetArrayItem` (`self.CameraActors`) (`self.CameraNum`)) 0.2 :!label _label_3) ; Switching Cameras
    )))

(event `Key|PageUp`
  (params (Key :type "Key Structure"))
  (:`Pressed`
    (if (!= (- (`KismetArrayLibrary.Array_Length` (`self.CameraActors`)) 1) (`self.CameraNum`))
      (set `self.CameraNum` (+ (`self.CameraNum`) 1))
      (goto _label_3))))

(event `self.ReceiveBeginPlay`
  (bind _returnvalue (`GameplayStatics.GetActorOfClass` "/Game/TeamShare/TeamShare_Kailra/Character/BP_TestAIC.BP_TestAIC_C"))
  (set `self.TestAIC` _returnvalue)
  (bind _returnvalue_2 (`GameplayStatics.GetActorOfClass` "/Game/TeamShare/TeamShare_Kailra/Stage/StageBase/BP_GridISM.BP_GridISM_C"))
  (bind _output_get (set `self.As BP GridISM` _returnvalue_2))
  (`/Engine/EditorBlueprintResources/StandardMacros.IsValid` _output_get
    (:`Is Valid`
      (`KismetSystemLibrary.K2_SetTimerDelegate` (delegate `MouseOverGrid`) 0.1 true)
      (bind _outactors (`GameplayStatics.GetAllActorsOfClass` "/Script/Engine.CameraActor"))
      (bind _output_get_2 (set `self.CameraActors` _outactors))
      (`self.SetViewTargetWithBlend` (`|GetArrayItem` _output_get_2 (`self.CameraNum`))) ; Set Camera
    )))

(event `MouseOverGrid`
  (bind (_bblockinghit _binitialoverlap _time _distance _location _impactpoint _normal _impactnormal _physmat _hitactor _hitcomponent _hitbonename _bonename _hititem) (`GameplayStatics.BreakHitResult` (`self.GetHitResultUnderCursorByChannel` "TraceTypeQuery3")))
  (if _bblockinghit
    (cast `/Game/TeamShare/TeamShare_Kailra/Stage/StageBase/BP_GridISM` _hitactor)
    (`/Game/TeamShare/TeamShare_Kailra/Stage/StageBase/BP_GridISM.MouseOverGrid` (`self.As BP GridISM`) _hititem)
    (else
      (`/Game/TeamShare/TeamShare_Kailra/Stage/StageBase/BP_GridISM.NotOverGrid` (`self.As BP GridISM`)))))

(fn `UserConstructionScript`)