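; BP_MouseOverGrid is a decal actor that highlights a grid spot, presumably the one under the mouse as its name suggests.
; VisibleGrid sets the decal's world scale to half the given size vector, moves the actor to the given grid location and unhides the decal.
; HiddenGrid hides the decal and also runs on BeginPlay, so the highlight starts hidden.
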(event `self.ReceiveBeginPlay`
  (`self.HiddenGrid`))

(event `VisibleGrid`
  (params (GridLocation :type "Vector Structure") (sizevector :type "Vector Structure"))
  (`SceneComponent.K2_SetWorldTransform` (`self.Decal`) (`KismetMathLibrary.MakeTransform` (0.0 0.0 0.0) (struct) (* sizevector 0.5)) false false)
  (`self.K2_SetActorLocation` GridLocation)
  (`SceneComponent.SetHiddenInGame` (`self.Decal`) false false))

(event `HiddenGrid`
  (`SceneComponent.SetHiddenInGame` (`self.Decal`) true false))

(fn `UserConstructionScript`)