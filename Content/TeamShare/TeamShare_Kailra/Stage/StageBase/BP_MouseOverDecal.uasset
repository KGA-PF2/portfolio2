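; BP_MouseOverDecal is a decal actor that marks a grid location with a highlight sized to a given vector, likely for mouse hover.
; It starts hidden on BeginPlay and is driven through two events, VisibleDecal and HiddenDecal.
; VisibleDecal sets the decal's world transform with half-size X/Y scale and a padded Z, moves the actor to the grid location and unhides it.
; HiddenDecal hides it again, with no Tick logic.
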(event `self.ReceiveBeginPlay`
  (`self.HiddenDecal`))

(event `VisibleDecal`
  (params (GridLocation :type "Vector Structure") (sizevector :type "Vector Structure"))
  (`SceneComponent.K2_SetWorldTransform` (`self.Decal`) (`KismetMathLibrary.MakeTransform` (0.0 0.0 0.0) (struct) (`KismetMathLibrary.MakeVector` (* (.x sizevector) 0.5) (* (.y sizevector) 0.5) (+ (.z sizevector) 0.2))) false false)
  (`self.K2_SetActorLocation` GridLocation)
  (`SceneComponent.SetHiddenInGame` (`self.Decal`) false false))

(event `HiddenDecal`
  (`SceneComponent.SetHiddenInGame` (`self.Decal`) true false))

(fn `UserConstructionScript`)