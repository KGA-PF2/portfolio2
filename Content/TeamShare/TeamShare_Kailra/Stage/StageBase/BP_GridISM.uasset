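; Grid actor for a stage that draws a tile grid with an instanced static mesh and supports mouse-over highlighting.
; BeginPlay stores the actor's location as the grid offset, then rebuilds plane instances in local space, scaled to leave gaps between cells.
; MouseOverGrid and NotOverGrid toggle the highlight through per-instance custom data read by the material.
; Getters expose grid layout and component, with helpers converting between instance index and X/Y coordinates.
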(event `self.ReceiveBeginPlay`
  (bind _gridinstance (`self.GridInstance`))
  (bind _gridinterval (`self.GridInterval`))
  ;[1 1 1] 오프셋 중요
  (set `self.GridLocationOffset` (`SceneComponent.K2_GetComponentLocation` (`self.DefaultSceneRoot`)))
  (`InstancedStaticMeshComponent.ClearInstances` _gridinstance) ; Reset
  (`StaticMeshComponent.SetStaticMesh` _gridinstance "/Engine/BasicShapes/Plane.Plane")
  (for _index (range (`self.GridWidth`))
    (for _index_2 (range (`self.GridHeight`))
      (`InstancedStaticMeshComponent.AddInstance` _gridinstance (`KismetMathLibrary.MakeTransform` (`KismetMathLibrary.MakeVector` (* _index (`self.GridSizeX`)) (* _index_2 (`self.GridSizeY`)) (`self.GridSizeZ`)) (struct) (`KismetMathLibrary.MakeVector` (/ (- (`self.GridSizeX`) _gridinterval) 100.0) (/ (- (`self.GridSizeY`) _gridinterval) 100.0) 1.0)) false))))

(event `MouseOverGrid`
  (params (FindIndex :type Integer))
  (set `self.NewItemIndex` FindIndex)
  (if (== (`self.NewItemIndex`) (`self.OldItemIndex`))
    (`InstancedStaticMeshComponent.SetCustomDataValue` (`self.GridInstance`) (`self.OldItemIndex`) 0 1.0 true) ; Conneted to Metarial *Instance - Custom Data Float*
    (else
      (`self.NotOverGrid`)
      (set `self.OldItemIndex` (`self.NewItemIndex`)))))

(event `NotOverGrid`
  (`InstancedStaticMeshComponent.SetCustomDataValue` (`self.GridInstance`) (`self.OldItemIndex`) 0 0.0 true))

(fn `GetGridCoordFromIndex`
  (params (Index :type Integer))
  (returns (ReturnValue :type "IntPoint Structure"))
  (bind _gridheight (`self.GridHeight`))
  (return (make `IntPoint` (/ Index _gridheight) (mod Index _gridheight))))

(fn `GetGridHeight`
  (returns (ReturnValue :type Integer))
  (return (`self.GridHeight`)))

(fn `GetGridIndexFromCoord`
  (params (Coord :type "IntPoint Structure"))
  (returns (ReturnValue :type Integer))
  (return (+ (* Coord_X (`self.GridHeight`)) Coord_Y)))

(fn `GetGridInstanceComponent`
  (returns (ReturnValue :type "InstancedStaticMeshComponent Object Reference"))
  (return (`self.GridInstance`)))

(fn `GetGridLocationOffset`
  (returns (ReturnValue :type "Vector Structure"))
  (return (`self.GridLocationOffset`)))

(fn `GetGridSizeX`
  (returns (ReturnValue :type "Float (double-precision)"))
  (return (`self.GridSizeX`)))

(fn `GetGridSizeY`
  (returns (ReturnValue :type "Float (double-precision)"))
  (return (`self.GridSizeY`)))

(fn `GetGridWidth`
  (returns (ReturnValue :type Integer))
  (return (`self.GridWidth`)))

(fn `UserConstructionScript`)