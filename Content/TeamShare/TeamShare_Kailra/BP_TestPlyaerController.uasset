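; Test player controller that switches between level cameras and drives mouse hover on an instanced-mesh grid.
; BeginPlay caches the grid and decal actors, gathers all CameraActors and sets the starting view; Left and Right keys step through them without index clamping.
; A looping 0.1-second timer, rather than Tick, traces under the cursor and passes the hit instance index to BP_GridISM, or clears hover on a miss.
; The decal show/hide calls are disconnected.
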(event `Key|Left`
  (params (Key :type "Key Structure"))
  (:`Pressed`
    (set `self.CameraNum` (- (`self.CameraNum`) 1))
    (`self.SetViewTargetWithBlend` (`|GetArrayItem` (`self.Out Actors`) (`self.CameraNum`)) :!label _label)))

(event `Key|Right`
  (params (Key :type "Key Structure"))
  (:`Pressed`
    (set `self.CameraNum` (+ (`self.CameraNum`) 1))
    (goto _label)))

(event `self.ReceiveBeginPlay`
  (`/Engine/EditorBlueprintResources/StandardMacros.IsValid` null
    (:`Is Valid`
      (bind _returnvalue (`GameplayStatics.GetActorOfClass` "/Game/TeamShare/TeamShare_Kailra/Stage/StageBase/BP_MouseOverDecal.BP_MouseOverDecal_C"))
      (set `self.As BP Mouse Over Grid` _returnvalue)
      (bind _returnvalue_2 (`GameplayStatics.GetActorOfClass` "/Game/TeamShare/TeamShare_Kailra/Stage/StageBase/BP_GridISM.BP_GridISM_C"))
      (set `self.As BP GridISM` _returnvalue_2)
      (`KismetSystemLibrary.K2_SetTimerDelegate` (delegate `MouseOverGrid`) 0.1 true)
      (bind _outactors (`GameplayStatics.GetAllActorsOfClass` "/Script/Engine.CameraActor"))
      (bind _output_get (set `self.Out Actors` _outactors))
      (`self.SetViewTargetWithBlend` (`|GetArrayItem` _output_get (`self.CameraNum`))))))

(event `MouseOverGrid`
  (bind (_bblockinghit _binitialoverlap _time _distance _location _impactpoint _normal _impactnormal _physmat _hitactor _hitcomponent _hitbonename _bonename _hititem) (`GameplayStatics.BreakHitResult` (`self.GetHitResultUnderCursorByChannel` "TraceTypeQuery3")))
  (if _bblockinghit
    (cast `/Game/TeamShare/TeamShare_Kailra/Stage/StageBase/BP_GridISM` _hitactor)
    (`/Game/TeamShare/TeamShare_Kailra/Stage/StageBase/BP_GridISM.MouseOverGrid` (`self.As BP GridISM`) _hititem)
    (else
      (`/Game/TeamShare/TeamShare_Kailra/Stage/StageBase/BP_GridISM.NotOverGrid` (`self.As BP GridISM`)))))

(fn `UserConstructionScript`)