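; BP_VFX_Container is a helper actor that spawns a one-shot particle effect in the world and then removes itself.
; SpawnParticleSimple spawns the emitter template at the location and rotation of a stored transform, multiplying its scale by VFXScale.
; It then calls VFXDestroySelf, which waits for VFXDuration and destroys the container actor.
; BeginPlay, overlap and Tick are empty, so spawning depends on an external call to SpawnParticleSimple.
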(event `VFXDestroySelf`
  (`KismetSystemLibrary.Delay` (`self.VFXDuration`))
  (`self.K2_DestroyActor` self))

(fn `SpawnParticle_Simple`
  (`GameplayStatics.SpawnEmitterAtLocation` (`self.Emitter Template`) (.location (`self.ParticleTranfrom`)) (.rotation (`self.ParticleTranfrom`)) (* (.scale (`self.ParticleTranfrom`)) (`self.VFXScale`)))
  (`self.VFXDestroySelf`))

(fn `UserConstructionScript`)