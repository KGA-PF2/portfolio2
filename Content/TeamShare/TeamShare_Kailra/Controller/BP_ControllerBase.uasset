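; BP_ControllerBase is a base player controller that provides pause-menu toggling and a game-over screen.
; SpawnMenu creates a widget of the given class and pauses the game, or unpauses and removes the current widget if one is stored in AsWidget.
; GameOver prints a debug string, passes WBP_GameOver through that same toggle, then switches input to UI only.
; BeginPlay and Tick are unused.
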(fn `GameOver`
  (`KismetSystemLibrary.PrintString` "Hello")
  (`self.SpawnMenu` "/Game/TeamShare/TeamShare_Kailra/UI/Pubilc/WBP_GameOver.WBP_GameOver_C")
  (`WidgetBlueprintLibrary.SetInputMode_UIOnlyEx` self null)
  (return))

(fn `SpawnMenu`
  (params (Class :type "UserWidget Class Reference"))
  (`/Engine/EditorBlueprintResources/StandardMacros.IsValid` (`self.As Widget`)
    (:`Is Valid`
      (`GameplayStatics.SetGamePaused` false)
      (`Widget.RemoveFromParent` (`self.As Widget`))
      (set `self.As Widget` null))
    (:`Is Not Valid`
      (`GameplayStatics.SetGamePaused` true)
      (bind _returnvalue (`|CreateWidget` Class))
      (bind _output_get (set `self.As Widget` _returnvalue))
      (`UserWidget.AddToViewport` _output_get 0))))

(fn `UserConstructionScript`)