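; Test player controller that drives a BP_TestAIC across a BP_GridISM_origin instanced grid using debug keys.
; Z, C and X pick the previous, next or random cell, while arrow keys step through calcTargetGridNum, sending cell locations to MovingOn.
; BeginPlay sets up input and gathers cameras for PageUp/PageDown blending; other inputs spawn pause and game-over menus.
; Grid lookup and the timed mouse-hover trace are disconnected, leaving the grid reference unassigned here.
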(event `Key|Z`
  (params (Key :type "Key Structure"))
  ;[1 1 1] Grid 순회 Z = -1, C = +1, X = Random
  (:`Pressed`
    (`/Engine/EditorBlueprintResources/StandardMacros.DecrementInt` (`self.InstanceIndexNum`)
      (:`  `
        (if (>= (`self.InstanceIndexNum`) 0.0)
          (`/Game/TeamShare/TeamShare_Kailra/Controller/BP_TestAIC.MovingOn` (`self.AS TestAIC`) (+ (.location (`InstancedStaticMeshComponent.GetInstanceTransform` (`/Game/TeamShare/TeamShare_Kailra/Stage/StageBase/BP_GridISM_origin.GridInstance` (`self.As BP GridISM`)) (`self.InstanceIndexNum`) false)) (`GridISM.GridLocationOffset` (`self.As BP GridISM`))) :!label _label)
          (else
            (set `self.InstanceIndexNum` 0)))))))

(event `MouseOverGrid`
  (bind (_bblockinghit _binitialoverlap _time _distance _location _impactpoint _normal _impactnormal _physmat _hitactor _hitcomponent _hitbonename _bonename _hititem) (`GameplayStatics.BreakHitResult` (`self.GetHitResultUnderCursorByChannel` "TraceTypeQuery3")))
  ;[1 1 1] Old Root
  (if _bblockinghit
    (cast `/Game/TeamShare/TeamShare_Kailra/Stage/StageBase/BP_GridISM_origin` _hitactor)
    (`/Game/TeamShare/TeamShare_Kailra/Stage/StageBase/BP_GridISM_origin.MouseOverGrid` (`self.As BP GridISM`) _hititem)
    (else
      (`/Game/TeamShare/TeamShare_Kailra/Stage/StageBase/BP_GridISM_origin.NotOverGrid` (`self.As BP GridISM`)))))

(event `Key|X`
  (params (Key :type "Key Structure"))
  (bind _as_bp_gridism (`self.As BP GridISM`))
  ;[1 1 1] Grid 순회 Z = -1, C = +1, X = Random
  (:`Pressed`
    (set `self.InstanceIndexNum` (`KismetMathLibrary.RandomIntegerInRange` 1 (- (* (`GridISM.GridWidth` _as_bp_gridism) (`GridISM.GridHeight` _as_bp_gridism)) 2)))
    (goto _label)))

(event `Key|C`
  (params (Key :type "Key Structure"))
  (bind _as_bp_gridism (`self.As BP GridISM`))
  (bind _returnvalue (- (* (`GridISM.GridWidth` _as_bp_gridism) (`GridISM.GridHeight` _as_bp_gridism)) 1))
  ;[1 1 1] Grid 순회 Z = -1, C = +1, X = Random
  (:`Pressed`
    (`/Engine/EditorBlueprintResources/StandardMacros.IncrementInt` (`self.InstanceIndexNum`)
      (:`  `
        (if (<= (`self.InstanceIndexNum`) _returnvalue)
          (goto _label)
          (else
            (set `self.InstanceIndexNum` _returnvalue)))))))

(event `Key|Up`
  (params (Key :type "Key Structure"))
  (bind _as_bp_gridism (`self.As BP GridISM`))
  ;[1 1 1] 이동 테스트
  (:`Pressed`
    (bind (_calcgridnum _bsuccessout) (`NewFunctionLibrary.CalcTargetGridNum` (`self.Current Grid Num`) (`GridISM.GridWidth` _as_bp_gridism) (`GridISM.GridHeight` _as_bp_gridism) :!label _label_2))
    (if _bsuccessout
      (set `self.Current Grid Num` _calcgridnum)
      (`/Game/TeamShare/TeamShare_Kailra/Controller/BP_TestAIC.MovingOn` (`self.AS TestAIC`) (`KismetMathLibrary.Conv_Vector2DToVector` (`KismetMathLibrary.Conv_VectorToVector2D` (+ (.location (`InstancedStaticMeshComponent.GetInstanceTransform` (`/Game/TeamShare/TeamShare_Kailra/Stage/StageBase/BP_GridISM_origin.GridInstance` (`self.As BP GridISM`)) (`self.Current Grid Num`) false)) (`GridISM.GridLocationOffset` (`self.As BP GridISM`)))))))))

(event `Key|Down`
  (params (Key :type "Key Structure"))
  ;[1 1 1] 이동 테스트
  (:`Pressed`
    (goto _label_2 :!via `Down`)))

(event `Key|Left`
  (params (Key :type "Key Structure"))
  ;[1 1 1] 이동 테스트
  (:`Pressed`
    (goto _label_2 :!via `Left`)))

(event `Key|Right`
  (params (Key :type "Key Structure"))
  ;[1 1 1] 이동 테스트
  (:`Pressed`
    (goto _label_2 :!via `Right`)))

(event `Key|PageDown`
  (params (Key :type "Key Structure"))
  (:`Pressed`
    (if (!= (+ (`KismetArrayLibrary.Array_Find` (`self.CameraActors`)) 1) (`self.CameraNum`))
      (set `self.CameraNum` (- (`self.CameraNum`) 1))
      (`self.SetViewTargetWithBlend` (`|GetArrayItem` (`self.CameraActors`) (`self.CameraNum`)) 0.2 :!label _label_3) ; Switching Cameras
    )))

(event `Key|PageUp`
  (params (Key :type "Key Structure"))
  (:`Pressed`
    (if (!= (- (`KismetArrayLibrary.Array_Length` (`self.CameraActors`)) 1) (`self.CameraNum`))
      (set `self.CameraNum` (+ (`self.CameraNum`) 1))
      (goto _label_3))))

(event `self.ReceiveBeginPlay`
  ;[1 1 1] 입력 설정
  (set `self.bShowMouseCursor` true)
  (`WidgetBlueprintLibrary.SetInputMode_GameAndUIEx` self null)
  (`EnhancedInputSubsystemInterface.AddMappingContext` (pcsubsystem `EnhancedInputLocalPlayerSubsystem` self) "/Game/TeamShare/TeamShare_JSH/Input/IMC_PlayerMove.IMC_PlayerMove" 0 (struct))
  ;[1 1 1] 카메라 설정
  (bind _outactors (`GameplayStatics.GetAllActorsOfClass` "/Script/Engine.CameraActor"))
  (bind _output_get (set `self.CameraActors` _outactors))
  (`self.SetViewTargetWithBlend` (`|GetArrayItem` _output_get (`self.CameraNum`))) ; Set Camera
  (bind _returnvalue (`GameplayStatics.GetActorOfClass` "/Game/TeamShare/TeamShare_Kailra/Controller/BP_TestAIC.BP_TestAIC_C"))
  (set `self.AS TestAIC` _returnvalue))

(event `EnhancedInput|/Game/TeamShare/TeamShare_JSH/Input/IA_PauseMenu`
  (params (ActionValue :type Boolean) (ElapsedSeconds :type "Float (double-precision)") (TriggeredSeconds :type "Float (double-precision)") (InputAction :type "InputAction Object Reference" :default "/Game/TeamShare/TeamShare_JSH/Input/IA_PauseMenu.IA_PauseMenu"))
  (:`Started`
    (`self.SpawnMenu` "/Game/TeamShare/TeamShare_Kailra/UI/PauseMenu/WBP_PauseMenu.WBP_PauseMenu_C")))

(event `Key|L`
  (params (Key :type "Key Structure"))
  (:`Released`
    (`self.SpawnMenu` "/Game/TeamShare/TeamShare_Kailra/UI/Pubilc/WBP_GameOver.WBP_GameOver_C")
    (`WidgetBlueprintLibrary.SetInputMode_UIOnlyEx` self null)))

(fn `SpawnPauseMenu`
  (`/Engine/EditorBlueprintResources/StandardMacros.IsValid` (`self.As Pause Menu`)
    (:`Is Valid`
      (`GameplayStatics.SetGamePaused` false)
      (`Widget.RemoveFromParent` (`self.As Pause Menu`))
      (set `self.As Pause Menu` null))
    (:`Is Not Valid`
      (`GameplayStatics.SetGamePaused` true)
      (bind _returnvalue (`|CreateWidget` "/Game/TeamShare/TeamShare_Kailra/UI/PauseMenu/WBP_PauseMenu.WBP_PauseMenu_C"))
      (bind _output_get (set `self.As Pause Menu` _returnvalue))
      (`UserWidget.AddToViewport` _output_get 0))))

(fn `UserConstructionScript`)